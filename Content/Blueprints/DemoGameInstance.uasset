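; Game instance Blueprint that handles online session hosting on dedicated servers and joining sessions.
; On Init, a dedicated server creates an advanced session without presence, then opens ThirdPersonExampleMap as a listen level on success.
; A custom join event takes a search result, joins that session and prints a Chinese success or failure message.
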(event Custom|Event_JoinGame
  (params (SearchResult :type Blueprint%20Session%20Result%20Structure%20%28by%20ref%29))
  (|JoinSession (Game|GetPlayerController 0) SearchResult
    (:OnSuccess
      (Development|PrintString "加入成功" true true "(R=0.000000,G=0.660000,B=1.000000,A=1.000000)" 1e+01))
    (:OnFailure
      (Development|PrintString "加入失败" true true "(R=0.000000,G=0.660000,B=1.000000,A=1.000000)" 1e+01))))

(event EventInit
  (bind _returnvalue (Networking|IsDedicatedServer))
  (Development|PrintString (Utilities|String|ToString(Boolean) _returnvalue) true true "(R=0.000000,G=0.660000,B=1.000000,A=1.000000)" 1e+01)
  (if _returnvalue
    (|AdvancedSession 0 (Game|GetPlayerController 0) 6 0 false true true false true true false false false true
      (:OnSuccess
        (Game|OpenLevel(byObjectReference) "/Game/GameMaps/ThirdPersonExampleMap.ThirdPersonExampleMap" true "listen")))))